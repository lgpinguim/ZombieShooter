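; Assault rifle weapon child Blueprint that adds automatic fire to the parent weapon's firing logic.
; BeginPlay pulls the rifle's ammo data from the game instance.
; WeaponFire fires once, then repeats on a looping timer, each shot calling parent fire, playing the gun animation and shell effect, and notifying the player character.
; An empty magazine stops fire and triggers the player's reload; StopFire clears the timer.
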(event `self.ReceiveBeginPlay`
  (`parent.ReceiveBeginPlay`)
  (bind _asfps_game_instance_bp (cast `/Game/Blueprints/FPS_GameInstance_BP` (`GameplayStatics.GetGameInstance`)))
  (set `self.AmmoData` (`/Game/Blueprints/FPS_GameInstance_BP.AssaultRifleAmmoData` _asfps_game_instance_bp)))

(event `self.WeaponFire`
  (params (FireType :type "/Game/Blueprints/Enums/FireType Enum" :default "NewEnumerator0"))
  (set `self.IsRifleFiring` true)
  (`self.RifleFire`)
  (bind _returnvalue (`KismetSystemLibrary.K2_SetTimerDelegate` (delegate `RifleFire`) (`self.AutomaticfireRate`) true))
  (set `self.RifleFireTimerHandler` _returnvalue))

(event `RifleFire`
  (bind (_returnvalue_location _returnvalue_rotation) (`KismetMathLibrary.BreakTransform` (`SceneComponent.GetSocketTransform` (`self.GunMesh`) "AmmoEject" "RTS_World")))
  (if (`self.IsRifleFiring`)
    (`parent.WeaponFire` (stale `self.WeaponFire` FireType))
    (`SkeletalMeshComponent.PlayAnimation` (`self.GunMesh`) "/Game/MilitaryWeapSilver/Weapons/Animations/Fire_Rifle_W.Fire_Rifle_W" false)
    (`GameplayStatics.SpawnEmitterAtLocation` "/Game/Particles/FX_Rifle_Shell.FX_Rifle_Shell" _returnvalue_location _returnvalue_rotation)
    (`/Game/Blueprints/FPS_Character_BP.CharacterFireWeapon` (`self.PlayerRef`) "NewEnumerator1")
    (if (<= (`self.CurrentAmmo`) 0)
      (`self.StopFire`)
      (`/Game/Blueprints/FPS_Character_BP.Reload` (`self.PlayerRef`)))))

(event `self.StopFire`
  (`parent.StopFire`)
  (set `self.IsRifleFiring` false)
  (`KismetSystemLibrary.K2_ClearAndInvalidateTimerHandle` (`self.RifleFireTimerHandler`)))

(fn `UserConstructionScript`
  (`parent.UserConstructionScript`))