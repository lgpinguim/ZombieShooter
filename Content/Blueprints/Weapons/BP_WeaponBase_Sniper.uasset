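; Sniper rifle child of the weapon base, adding scoped aiming and its own fire effects.
; BeginPlay pulls sniper ammo data from the game instance, and firing plays the gun animation and ejects a shell emitter at the AmmoEject socket.
; Aiming in blocks weapon switching and reloading, then after a short delay shows the scope widget while hiding the gun, player pawn and main HUD.
; Aiming out reverses this.
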(event `self.ReceiveBeginPlay`
  (`parent.ReceiveBeginPlay`)
  (bind _asfps_game_instance_bp (cast `/Game/Blueprints/FPS_GameInstance_BP` (`GameplayStatics.GetGameInstance`)))
  (set `self.AmmoData` (`/Game/Blueprints/FPS_GameInstance_BP.SniperRifleAmmoData` _asfps_game_instance_bp)))

(event `self.WeaponFire`
  (params (FireType :type "/Game/Blueprints/Enums/FireType Enum" :default "NewEnumerator0"))
  (bind _gunmesh (`self.GunMesh`))
  (bind (_returnvalue_location _returnvalue_rotation) (`KismetMathLibrary.BreakTransform` (`SceneComponent.GetSocketTransform` _gunmesh "AmmoEject" "RTS_World")))
  (`parent.WeaponFire` FireType)
  (`SkeletalMeshComponent.PlayAnimation` _gunmesh "/Game/MilitaryWeapSilver/Weapons/Animations/Fire_SniperRifle_W.Fire_SniperRifle_W" false)
  (`GameplayStatics.SpawnEmitterAtLocation` "/Game/Particles/FX_SniperRifle_Shell.FX_SniperRifle_Shell" _returnvalue_location _returnvalue_rotation))

(event `self.OnAimEnter`
  (bind _playerref (`self.PlayerRef`))
  (bind _sniperscoperef (`/Game/Blueprints/FPS_Character_BP.SniperScopeRef` (`self.PlayerRef`)))
  (`parent.OnAimEnter`)
  (if (== (`/Game/Blueprints/FPS_Character_BP.CurrentWeapon` (`self.PlayerRef`)) self)
    (set `/Game/Blueprints/FPS_Character_BP.CanSwitchWeapon` false _playerref)
    (set `/Game/Blueprints/FPS_Character_BP.CanReload` false _playerref)
    (`KismetSystemLibrary.Delay` 0.1)
    (if (not (`Widget.IsInViewport` _sniperscoperef))
      (`UserWidget.AddToViewport` _sniperscoperef 0)
      (`SceneComponent.SetHiddenInGame` (`self.GunMesh`) true false)
      (`self.SetActorHiddenInGame` (`GameplayStatics.GetPlayerPawn` 0) true)
      (`Widget.SetVisibility` (`/Game/Blueprints/FPS_Character_BP.MainHudRef` (`self.PlayerRef`)) "Collapsed"))))

(event `self.OnAimExit`
  (bind _playerref (`self.PlayerRef`))
  (`parent.OnAimExit`)
  (set `/Game/Blueprints/FPS_Character_BP.CanSwitchWeapon` true _playerref)
  (set `/Game/Blueprints/FPS_Character_BP.CanReload` true _playerref)
  (`Widget.RemoveFromParent` (`/Game/Blueprints/FPS_Character_BP.SniperScopeRef` (`self.PlayerRef`)))
  (`SceneComponent.SetHiddenInGame` (`self.GunMesh`) false false)
  (`self.SetActorHiddenInGame` (`GameplayStatics.GetPlayerPawn` 0) false)
  (`Widget.SetVisibility` (`/Game/Blueprints/FPS_Character_BP.MainHudRef` (`self.PlayerRef`)) "Visible"))

(fn `UserConstructionScript`
  (`parent.UserConstructionScript`))