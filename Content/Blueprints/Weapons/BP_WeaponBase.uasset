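; Base weapon Blueprint that handles hitscan firing, magazine and reserve ammo, and recoil for the player's guns.
; WeaponFire spends ammo and runs one or several camera line traces with random spread, ending at forward times range without the camera location added.
; Each trace spawns an impact effect and sends damage data to the hit actor via TakeDamageMessage.
; Automatic weapons add timeline-driven pitch kick with random yaw, then reverse the pitch.
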(event `self.ReceiveBeginPlay`
  (bind _asfps_character_bp (cast `/Game/Blueprints/FPS_Character_BP` (`GameplayStatics.GetPlayerPawn` 0)))
  (set `self.PlayerRef` _asfps_character_bp))

(event `AutomaticRecoil`
  (bind _returnvalue (`GameplayStatics.GetPlayerPawn` 0))
  (bind (_direction _alpha) (`Timeline|RecoilTimeline` :!via `PlayFromStart` :!label _label)
    (:`Update`
      (switch `ETimelineDirection` _direction
        (:`Forward`
          (bind _returnvalue_2 (`KismetMathLibrary.Lerp` 0.0 (`self.RecoilPitch`) _alpha))
          (`Pawn.AddControllerPitchInput` _returnvalue _returnvalue_2)
          (`Pawn.AddControllerYawInput` _returnvalue (`KismetMathLibrary.RandomFloatInRange` -0.3 0.3)))
        (:`Backward`
          (`Pawn.AddControllerPitchInput` _returnvalue (* _returnvalue_2 -1.0)))))
    (:`Finished`
      (`self.ReverseRecoil`)
      (`KismetSystemLibrary.RetriggerableDelay` 0.05)
      (`self.StopRecoil`))))

(event `StopRecoil`
  (goto _label :!via `Stop`))

(event `ReverseRecoil`
  (goto _label :!via `Reverse`))

(fn `AddDamage`
  (params (HitResult :type "HitResult Structure"))
  (message `/Game/Blueprints/Interfaces/TakeDamage.TakeDamage` (`.HitActor` (`GameplayStatics.BreakHitResult` HitResult)) (`self.AmmoData`) (`self.CriticalHitModifier`) HitResult))

(fn `CalculateShot`
  (params (Camera :type "CameraComponent Object Reference") (WeaponMesh :type "SceneComponent Object Reference") (WeaponFireSocketName :type Name))
  (returns (HitResult :type "HitResult Structure"))
  (locals (`Local Camera` :type "CameraComponent Object Reference") (`Local Weapon Mesh` :type "SceneComponent Object Reference") (`Local Socket Name` :type Name))
  (bind _bulletspread (`self.BulletSpread`))
  (bind (_returnvalue_location _returnvalue_rotation) (`KismetMathLibrary.BreakTransform` (`SceneComponent.K2_GetComponentToWorld` (`local.Local Camera`))))
  (bind _returnvalue (* _bulletspread -1.0))
  (bind (_returnvalue_x _returnvalue_y _returnvalue_z) (`KismetMathLibrary.BreakVector` (+ (0.0 0.0 0.0) (* (`KismetMathLibrary.GetForwardVector` _returnvalue_rotation) (`self.WeaponRange`)))))
  (`|ExecutionSequence`
    (:`then_0`
      (set `local.Local Camera` Camera)
      (set `local.Local Weapon Mesh` WeaponMesh)
      (set `local.Local Socket Name` WeaponFireSocketName))
    (:`then_1`
      (bind _outhit (`KismetSystemLibrary.LineTraceSingleForObjects` _returnvalue_location (`KismetMathLibrary.MakeVector` (+ _returnvalue_x (`KismetMathLibrary.RandomFloatInRange` _returnvalue _bulletspread)) (+ _returnvalue_y (`KismetMathLibrary.RandomFloatInRange` _returnvalue _bulletspread)) (+ _returnvalue_z (`KismetMathLibrary.RandomFloatInRange` _returnvalue _bulletspread))) (`|MakeArray` "ObjectTypeQuery1" "ObjectTypeQuery2" :!type "EObjectTypeQuery Enum") false (`|MakeArray` (`GameplayStatics.GetPlayerPawn` 0) null :!type "Actor Object Reference")))
      (return _outhit))))

(fn `HasAmmoInMag`
  (returns (HasAmmo :type Boolean) (MagFull :type Boolean))
  (return (> (`self.CurrentAmmo`) 0) (== (`self.MaxMagAmmo`) (`self.CurrentAmmo`))))

(fn `HasExtraAmmo`
  (returns (`Has Extra Ammo` :type Boolean))
  (return (> (`self.CurrentTotalAmmo`) 0)))

(fn `StopFire`)

(fn `UserConstructionScript`)

(fn `WeaponFire`
  (set `self.CurrentAmmo` (- (`self.CurrentAmmo`) 1))
  (if (`self.HasMultipleBullets`)
    (for _ (range (`self.BulletCount`))
      (bind _hitresult (`self.CalculateShot` (`/Game/Blueprints/FPS_Character_BP.Camera` (`self.PlayerRef`)) (`self.GunMesh`) "MuzzleFlash" :!label _label))
      (bind (_bblockinghit _binitialoverlap _time _distance _location _impactpoint) (`GameplayStatics.BreakHitResult` _hitresult))
      (`|SpawnActorFromClass` (`self.ImpactEffectClass`) (`KismetMathLibrary.MakeTransform` _impactpoint) "Undefined" "OverrideRootScale" null _hitresult _bblockinghit null)
      (`self.AddDamage` _hitresult)
      (if (`self.IsAutomaticWeapon`)
        (`self.AutomaticRecoil`)))
    (else
      (goto _label))))

(fn `WeaponReload`
  (bind _returnvalue (`KismetMathLibrary.Min` (`self.MaxMagAmmo`) (`self.CurrentTotalAmmo`)))
  (set `self.CurrentAmmo` _returnvalue)
  (set `self.CurrentTotalAmmo` (- _returnvalue (`self.CurrentTotalAmmo`))))