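; Pistol weapon Blueprint that adds pistol-specific ammo data and firing effects to its parent weapon class.
; On BeginPlay it copies the pistol ammo data from FPS_GameInstance_BP into its AmmoData variable.
; Firing runs the parent logic, plays the gun mesh fire animation and spawns a shell particle at the AmmoEject socket.
; Reload only calls the parent implementation.
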(event `self.ReceiveBeginPlay`
  (`parent.ReceiveBeginPlay`)
  (bind _asfps_game_instance_bp (cast `/Game/Blueprints/FPS_GameInstance_BP` (`GameplayStatics.GetGameInstance`)))
  (set `self.AmmoData` (`/Game/Blueprints/FPS_GameInstance_BP.PistolAmmoData` _asfps_game_instance_bp)))

(event `self.WeaponFire`
  (bind (_returnvalue_location _returnvalue_rotation) (`KismetMathLibrary.BreakTransform` (`SceneComponent.GetSocketTransform` (`self.GunMesh`) "AmmoEject" "RTS_World")))
  (`parent.WeaponFire`)
  (`SkeletalMeshComponent.PlayAnimation` (`self.GunMesh`) "/Game/MilitaryWeapSilver/Weapons/Animations/Fire_Pistol_W.Fire_Pistol_W" false)
  (`GameplayStatics.SpawnEmitterAtLocation` "/Game/Particles/FX_Pistol_Shell.FX_Pistol_Shell" _returnvalue_location _returnvalue_rotation))

(event `self.WeaponReload`
  (`parent.WeaponReload`))

(fn `UserConstructionScript`
  (`parent.UserConstructionScript`))